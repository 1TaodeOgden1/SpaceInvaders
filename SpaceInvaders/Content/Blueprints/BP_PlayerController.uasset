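; BP_PlayerController is the player controller that handles side-to-side movement and shooting for the player ship.
; On BeginPlay it adds the IM_PlayerControls Enhanced Input mapping context.
; Left and Right actions feed movement input along the world Y axis to the controlled pawn.
; Shoot spawns BP_Projectile at the BP_PlayerShip location, using a CanShoot flag and Delay as a half-second cooldown.
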(event Input|EnhancedActionEvents|EnhancedInputActionLeft
  (params (ActionValue :type Float%20%28double-precision%29) (ElapsedSeconds :type Float%20%28double-precision%29) (TriggeredSeconds :type Float%20%28double-precision%29) (InputAction :type Input%20Action%20Object%20Reference :default "/Game/Input/Left.Left"))
  ;[1 1 1] Input Actions for Left and Right (Movement is a little slidy at the moment)
  (Pawn|Input|AddMovementInput (Pawn|GetControlledPawn) "0.000000,-1.000000,0.000000" 1.0 false))

(event Input|EnhancedActionEvents|EnhancedInputActionRight
  (params (ActionValue :type Float%20%28double-precision%29) (ElapsedSeconds :type Float%20%28double-precision%29) (TriggeredSeconds :type Float%20%28double-precision%29) (InputAction :type Input%20Action%20Object%20Reference :default "/Game/Input/Right.Right"))
  ;[1 1 1] Input Actions for Left and Right (Movement is a little slidy at the moment)
  (Pawn|Input|AddMovementInput (Pawn|GetControlledPawn) "0.000000,1.000000,0.000000" 1.0 false))

(event Input|EnhancedActionEvents|EnhancedInputActionShoot
  (params (ActionValue :type Float%20%28double-precision%29) (ElapsedSeconds :type Float%20%28double-precision%29) (TriggeredSeconds :type Float%20%28double-precision%29) (InputAction :type Input%20Action%20Object%20Reference :default "/Game/Input/Shoot.Shoot"))
  ;[1 1 1] Shooting
  (if (Variables|Default|GetCanShoot)
    (bind _asbp_player_ship (Utilities|Casting|CastToBP_PlayerShip (Pawn|GetControlledPawn)))
    (Game|SpawnActorfromClass "/Game/Entities/BP_Projectile.BP_Projectile_C" (Math|Transform|MakeTransform (Transformation|GetActorLocation _asbp_player_ship) "0, 0, 0" "1.000000,1.000000,1.000000") "Undefined" "MultiplyWithRoot" 0 0)
    (Variables|Default|SetCanShoot false)
    (Utilities|FlowControl|Delay 0.5)
    (Variables|Default|SetCanShoot true)))

(event EventBeginPlay
  ;[1 1 1] Set up Input Action Mapping Context
  (Input|AddMappingContext (PlayerController|LocalPlayerSubsystems|GetEnhancedInputLocalPlayerSubsystem) "/Game/Input/IM_PlayerControls.IM_PlayerControls" 0 "(bIgnoreAllPressedKeysUntilRelease=True,bForceImmediately=False,bNotifyUserSettings=False)"))

(fn ConstructionScript)