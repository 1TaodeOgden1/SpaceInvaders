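; BP_AlienProjectile is an alien shot that travels straight down along Z until it hits something or expires.
; Tick moves it by a fixed step each frame without delta-time scaling, and the construction script sets its lifespan.
; On overlap, it switches on the other actor's first tag: Player and Fort actors are cast and damaged before the projectile destroys itself, while Base Bound just destroys it.
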(event Collision|EventActorBeginOverlap
  (params (OtherActor :type Actor%20Object%20Reference))
  (bind _tags (Variables|/Script/Engine.Actor|GetTags OtherActor))
  ;[1 1 1] check for collisions from relevant objects such as the player or a fort
  (if (Utilities|Array|IsValidIndex _tags)
    (switch name (Utilities|Array|Get(acopy) _tags)
      (:BaseBound
        _)
      (:Player
        (bind _asbp_player_ship (Utilities|Casting|CastToBP_PlayerShip OtherActor))
        (Default|TakeHit _asbp_player_ship))
      (:Fort
        (bind _asbp_fort (Utilities|Casting|CastToBP_Fort OtherActor))
        (Default|TakeDamage _asbp_fort)))
    (Actor|DestroyActor)))

(event EventBeginPlay)

(event EventTick
  (params (DeltaSeconds :type Float%20%28single-precision%29))
  (bind _returnvalue (Transformation|GetActorLocation))
  (Transformation|SetActorLocation (Math|Vector|MakeVector (.x _returnvalue) (.y _returnvalue) (+ (.z _returnvalue) -2.5)) false false))

(fn ConstructionScript
  ;[1 1 1] lifespan
  (Actor|SetLifeSpan 8.0))