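; BP_Exploder is an alien enemy that explodes and removes itself when hits bring its health to zero.
; Explode runs a box trace around the actor, sized by ExplodeRadius and briefly debug-drawn, then branches on each hit actor's first tag.
; It damages a player ship, alien or fort through a cast, returning after the first such hit rather than damaging everything in range.
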(event Collision|EventActorBeginOverlap
  (params (OtherActor :type Actor%20Object%20Reference))
  (|CallParentFunction OtherActor))

(event EventTakeHit
  (bind _health (Variables|Default|GetHealth))
  (Math|Integer|DecrementInt _health
    (:%20%20
      (if (<= _health 0)
        (Utilities|Explode)
        (CallFunction|RemoveAlien)))))

(fn ConstructionScript
  (|CallParentFunction))