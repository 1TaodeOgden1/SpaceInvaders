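; BP_AlienWave is an actor that tracks a wave of aliens and removes itself once all of them are dead.
; AlienKilled removes the dead alien from AlienList and fires NoAliensLeft when the list is empty, which destroys the wave actor.
; BeginPlay loops over InitialCount with an empty body, so nothing here spawns aliens or fills the list, and the construction script is empty.
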(event Custom|NoAliensLeft
  (Actor|DestroyActor))

(event Custom|AlienKilled
  (params (dead%20alien :type BP%20Alien%20Object%20Reference))
  (Utilities|Array|RemoveItem (Variables|Default|GetalienList) dead%20alien)
  (if (<= (Utilities|Array|Length (Variables|Default|GetalienList)) 0)
    (CallFunction|NoAliensLeft)))

(event EventBeginPlay
  (for _index (range 0 (Variables|Default|GetinitialCount))
    _))

(fn ConstructionScript)