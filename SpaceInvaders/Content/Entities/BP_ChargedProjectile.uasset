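; BP_ChargedProjectile is a charged shot that travels upward along Z by a fixed, frame-rate-dependent step each Tick.
; Overlaps destroy it at top bounds; otherwise it calls TakeHit on enemy aliens and plays a non-looping explosion flipbook.
; When a flipbook finishes, it switches back to the travel flipbook without destroying the actor, so the shot survives hits.
; The construction script sets a lifespan as a cleanup fallback.
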(event OnFinishedPlaying(sprite)
  (Sprite|SetFlipbook (Variables|Default|Getsprite) "/Game/Sprites/Bullets/FP_Bullet_travel.FP_Bullet_travel"))

(event Collision|EventActorBeginOverlap
  (params (OtherActor :type Actor%20Object%20Reference))
  ;[1 1 1] check for collisions from relevant objects; if the collision is with an alien, we tell it to react accordingly
  (if (Actor|ActorHasTag OtherActor "topBounds")
    (Actor|DestroyActor)
    (else
      (if (Actor|ActorHasTag OtherActor "Enemy")
        (bind _asbp_alien (Utilities|Casting|CastToBP_Alien OtherActor))
        (Default|TakeHit _asbp_alien))
      ;[1 1 1] play explosion animation
      (Sprite|SetFlipbook (Variables|Default|Getsprite) "/Game/Sprites/Bullets/FP_Bullet_Explosion.FP_Bullet_Explosion")
      ;[1 1 1] Allows OnFinishedPlaying event to trigger (which destroys the actor)
      (Components|Timeline|SetLooping (Variables|Default|Getsprite) false))))

(event EventTick
  (params (DeltaSeconds :type Float%20%28single-precision%29))
  (bind _returnvalue (Transformation|GetActorLocation))
  ;[1 1 1] Basic Projectile Movement
  (if (not (Variables|Default|GettoBeDestroyed))
    (Transformation|SetActorLocation (Math|Vector|MakeVector (.x _returnvalue) (.y _returnvalue) (+ (.z _returnvalue) 2.0)) false false)))

(fn ConstructionScript
  ;[1 1 1] lifespan
  (Actor|SetLifeSpan 8.0))