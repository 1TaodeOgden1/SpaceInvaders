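; BP_Fort is a destructible fort, using Space Invaders sprites, that shows its remaining durability as text.
; Each TakeDamage event decrements Durability and switches on the result, stepping through four Paper2D damage sprites in paired durability bands, or destroying the actor at zero.
; SetDisplayText refreshes the durability label on BeginPlay and after each sprite update.
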(event Custom|TakeDamage
  (bind _papersprite (Variables|Default|GetPaperSprite))
  (bind _result (Math|Integer|DecrementInt (Variables|Default|Getdurability))
    (:%20%20
      (switch int _result
        (:0
          (Actor|DestroyActor))
        (:1
          (Rendering|Components|Sprite|SetSprite _papersprite "/Game/Sprites/Forts/SpaceInvaders_sprites_scaled_Sprite_3.SpaceInvaders_sprites_scaled_Sprite_3" :!label _label)
          (Utilities|SetDisplayText :!label _label_2))
        (:2
          (goto _label))
        (:3
          (Rendering|Components|Sprite|SetSprite _papersprite "/Game/Sprites/Forts/SpaceInvaders_sprites_scaled_Sprite_2.SpaceInvaders_sprites_scaled_Sprite_2" :!label _label_3)
          (goto _label_2))
        (:4
          (goto _label_3))
        (:5
          (Rendering|Components|Sprite|SetSprite _papersprite "/Game/Sprites/Forts/SpaceInvaders_sprites_scaled_Sprite_1.SpaceInvaders_sprites_scaled_Sprite_1" :!label _label_4)
          (goto _label_2))
        (:6
          (goto _label_4))
        (:7
          (Rendering|Components|Sprite|SetSprite _papersprite "/Game/Sprites/Forts/SpaceInvaders_sprites_scaled_Sprite_0.SpaceInvaders_sprites_scaled_Sprite_0" :!label _label_5)
          (goto _label_2))
        (:8
          (goto _label_5))))))

(event EventBeginPlay
  (Utilities|SetDisplayText))

(event EventTick
  (params (DeltaSeconds :type Float%20%28single-precision%29)))

(fn ConstructionScript)