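; BP_PlayerShip is the player's ship, which fires projectiles with a cooldown between shots.
; Shoot calls ShootBullet, which spawns a BP_Projectile at the ProjectileSpawn component's location when CanShoot is true.
; Shoot then calls the FiredProjectile event, which clears CanShoot and restores it after a ShootCooldown delay.
; The Move function and construction script are empty.
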(event Custom|FiredProjectile
  (Variables|Default|SetCanShoot false)
  (Utilities|FlowControl|Delay (Variables|Default|GetshootCooldown))
  (Variables|Default|SetCanShoot true))

(fn ConstructionScript)

(fn Move)

(fn Shoot
  (Utilities|ShootBullet)
  (CallFunction|FiredProjectile))