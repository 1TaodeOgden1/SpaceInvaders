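; BP_Alien is an enemy in a wave-based alien shooter that reports its boundary contacts and death to its owning wave.
; Overlaps with actors tagged as left or right bounds notify OwningWave of the edge hit.
; TakeHit adds score to the BP_PlayerShip player character and tells the wave this alien was killed, leaving any removal or movement response to the wave.
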(event Custom|Take%20Hit
  (bind _asbp_player_ship (Utilities|Casting|CastToBP_PlayerShip (Game|GetPlayerCharacter 0)))
  (Variables|/Game/Entities/BP_PlayerShip.BP_PlayerShip_C|SetScore _asbp_player_ship (+ (Variables|/Game/Entities/BP_PlayerShip.BP_PlayerShip_C|GetScore _asbp_player_ship) 100))
  (Default|AlienKilled (Variables|Default|Getowning_wave) self))

(event Collision|EventActorBeginOverlap
  (params (OtherActor :type Actor%20Object%20Reference))
  (if (Actor|ActorHasTag OtherActor "LeftBound")
    (Default|HitLeftBound (Variables|Default|Getowning_wave))
    (elif (Actor|ActorHasTag OtherActor "Rightbound")
      (Default|HitRightBound (Variables|Default|Getowning_wave)))))

(fn ConstructionScript)